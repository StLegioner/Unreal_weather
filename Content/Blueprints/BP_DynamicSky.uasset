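; Sky actor that sets sun, moon, stars, atmosphere and clouds from a TimeOfDay value.
; All work runs in the Construction Script, with no active Tick, so the sky does not advance by itself.
; Time relative to dawn and dusk drives light rotation and visibility, night atmosphere values and star and moon fades on a dynamic sky-sphere material.
; CurrentCloudMode selects no clouds, 2D sky-material clouds or a volumetric cloud component.
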(event EventBeginPlay)

(event Collision|EventActorBeginOverlap
  (params (OtherActor :type Actor%20Object%20Reference)))

(event EventTick
  (params (DeltaSeconds :type Float%20%28single-precision%29)))

(fn ConstructionScript
  (bind _returnvalue (Rendering|Material|CreateDynamicMaterialInstance (Variables|Default|GetSM_SkySphere) 0 "/Game/Materials/Sky/MI_DynamicSkySphere.MI_DynamicSkySphere" "None" :!class /Script/Engine.PrimitiveComponent))
  (Variables|Default|SetCreatedDynamicMISkySpere _returnvalue)
  (Utilities|FlowControl|Sequence
    (:then_1
      (01-BasicSettings|Sun/MoonRotationControl))
    (:then_2
      (01-BasicSettings|Sun/MoonVisibilityControl))
    (:then_3
      (02-NightSettings|NightSettingsControl))
    (:then_4
      (CallFunction|HandleCloudSettings))))

(fn Sun/MoonRotationControl
  ;[1 1 1] Sun control
  (Transformation|SetWorldRotation (Variables|Default|GetSunDirectionalLight) (Math|Rotator|MakeRotator 0.0 (Math|Float|MapRangeUnclamped (Variables|01-BasicSettings|GetTimeOfDay) (Variables|01-BasicSettings|GetDawnTime) (Variables|01-BasicSettings|GetDuskTime) 0.0 -1.8e+02) (Variables|01-BasicSettings|GetSunMoonRotation)) false false)
  (if (> (Variables|01-BasicSettings|GetTimeOfDay) 15.0)
    ;[1 1 1] Moon control from dusk till Midnight
    (Transformation|SetWorldRotation (Variables|Default|GetMoonDirectionalLight) (Math|Rotator|MakeRotator 0.0 (Math|Float|MapRangeUnclamped (Variables|01-BasicSettings|GetTimeOfDay) (+ (Variables|01-BasicSettings|GetDuskTime) (Variables|01-BasicSettings|GetDay/NightShift)) 24.0 0.0 -9e+01) (Variables|01-BasicSettings|GetSunMoonRotation)) false false)
    (else
      ;[1 1 1] Moon control from midnight till dawn
      (Transformation|SetWorldRotation (Variables|Default|GetMoonDirectionalLight) (Math|Rotator|MakeRotator 0.0 (Math|Float|MapRangeUnclamped (Variables|01-BasicSettings|GetTimeOfDay) 0.0 (- (Variables|01-BasicSettings|GetDawnTime) (Variables|01-BasicSettings|GetDay/NightShift)) -9e+01 -1.8e+02) (Variables|01-BasicSettings|GetSunMoonRotation)) false false))))

(fn Sun/MoonVisibilityControl
  (Rendering|SetVisibility (Variables|Default|GetSunDirectionalLight) (Utilities|IsDayTime) false)
  (Rendering|SetVisibility (Variables|Default|GetMoonDirectionalLight) (Utilities|IsNightTime) false))

(fn NightSettingsControl
  (bind _day_nightshift (Variables|01-BasicSettings|GetDay/NightShift))
  (bind _dusktime (Variables|01-BasicSettings|GetDuskTime))
  (bind _day_nightshift_2 (Variables|01-BasicSettings|GetDay/NightShift))
  (bind _dawntime (Variables|01-BasicSettings|GetDawnTime))
  (bind _dusktime_2 (Variables|01-BasicSettings|GetDuskTime))
  (bind _returnvalue (+ _dusktime _day_nightshift_2 0.0))
  (bind _returnvalue_2 (- _dawntime _day_nightshift))
  (Utilities|FlowControl|Sequence
    (:then_0
      (if (Utilities|IsNightTime)
        (Utilities|FlowControl|Sequence
          (:then_0
            (Rendering|Components|Light|SetIntensity (Variables|Default|GetMoonDirectionalLight) (Variables|02-NightSettings|GetMoonLightIntencity))
            (Rendering|Components|Light|SetLightColor (Variables|Default|GetMoonDirectionalLight) (Variables|02-NightSettings|GetMoonLightColor) true)
            (Class|LightComponent|SetTemperature (Variables|Default|GetMoonDirectionalLight) (Variables|02-NightSettings|GetMoonLightTemperature))
            (Class|DirectionalLightComponent|SetLightSourceAngle (Variables|Default|GetMoonDirectionalLight) (Variables|02-NightSettings|GetMoonLightAngle)))
          (:then_1
            (Class|SkyAtmosphereComponent|SetRayleighScattering (Variables|Default|GetSkyAtmosphere) (Variables|02-NightSettings|GetNighttimeRayleighScattering))
            (Class|SkyAtmosphereComponent|SetMultiScatteringFactor (Variables|Default|GetSkyAtmosphere) (Variables|02-NightSettings|GetNighttime%20Multi%20Scattering))
            (Class|SkyAtmosphereComponent|SetGroundAlbedo (Variables|Default|GetSkyAtmosphere) (Variables|02-NightSettings|GetNighttimeGroundAlbedo))))
        (else
          (Class|SkyAtmosphereComponent|SetRayleighScattering (Variables|Default|GetSkyAtmosphere) "(R=0.174647,G=0.407240,B=1.000000,A=1.000000)")
          (Class|SkyAtmosphereComponent|SetMultiScatteringFactor (Variables|Default|GetSkyAtmosphere) 0.5)
          (Class|SkyAtmosphereComponent|SetGroundAlbedo (Variables|Default|GetSkyAtmosphere) (LocalVariables|GetDefaultGroundAlbedo)))))
    (:then_1
      ;[1 1 1] Stars and moon visibility control
      (if (> (Variables|01-BasicSettings|GetTimeOfDay) (- (Variables|01-BasicSettings|GetDuskTime) 2.0))
        (Rendering|Material|SetScalarParameterValue (Variables|Default|GetCreatedDynamicMISkySpere) "StarsVisibility" (Math|Float|MapRangeClamped (Variables|01-BasicSettings|GetTimeOfDay) (- _dusktime_2 1.0) (+ _dusktime_2 (Variables|01-BasicSettings|GetDay/NightShift)) 0.0 1.0) :!class /Script/Engine.MaterialInstanceDynamic)
        (Rendering|Material|SetScalarParameterValue (Variables|Default|GetCreatedDynamicMISkySpere) "MoonVisibility" (Math|Float|MapRangeClamped (Variables|01-BasicSettings|GetTimeOfDay) _returnvalue (+ _returnvalue 0.1) 0.0 1.0) :!class /Script/Engine.MaterialInstanceDynamic)
        (else
          (Rendering|Material|SetScalarParameterValue (Variables|Default|GetCreatedDynamicMISkySpere) "StarsVisibility" (Math|Float|MapRangeClamped (Variables|01-BasicSettings|GetTimeOfDay) (- (Variables|01-BasicSettings|GetDawnTime) (Variables|01-BasicSettings|GetDay/NightShift)) (+ (Variables|01-BasicSettings|GetDawnTime) 1.0) 1.0 0.0) :!class /Script/Engine.MaterialInstanceDynamic)
          (Rendering|Material|SetScalarParameterValue (Variables|Default|GetCreatedDynamicMISkySpere) "MoonVisibility" (Math|Float|MapRangeClamped (Variables|01-BasicSettings|GetTimeOfDay) (- _returnvalue_2 0.1) _returnvalue_2 1.0 0.0) :!class /Script/Engine.MaterialInstanceDynamic))))
    (:then_2
      ;[1 1 1] Moon Visibility Control
      (Rendering|Material|SetVectorParameterValue (Variables|Default|GetCreatedDynamicMISkySpere) "MoonBasicSettings" (Utilities|Struct|MakeLinearColor (/ (Variables|02-NightSettings|GetMoon%20Scale) 5.0) (Variables|02-NightSettings|GetMoonRotation) (Variables|02-NightSettings|GetMoonBrightness) 1.0) :!class /Script/Engine.MaterialInstanceDynamic)
      (Rendering|Material|SetVectorParameterValue (Variables|Default|GetCreatedDynamicMISkySpere) "MoonTint" (Variables|02-NightSettings|GetMoonTint) :!class /Script/Engine.MaterialInstanceDynamic))))

(fn HandleCloudSettings
  (switch Utilities|FlowControl|Switch|SwitchonECloudMode (Variables|03-CloudSettings|GetCurrentCloudMode)
    (:NewEnumerator0
      (Utilities|Toggle2DClouds false)
      (Utilities|ToggleVolumetricCloud false))
    (:NewEnumerator1
      (Utilities|Toggle2DClouds true)
      (Utilities|Set2DCloudsSettings)
      (Utilities|ToggleVolumetricCloud false))
    (:NewEnumerator2
      (Utilities|Toggle2DClouds false)
      (Utilities|ToggleVolumetricCloud true)
      (Utilities|SetVolumetricCloudSettings))))